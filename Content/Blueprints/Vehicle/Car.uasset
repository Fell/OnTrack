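; Car actor that rides along the spline of a referenced Track, starting at BeginPlay when IsActive is set.
; The Mover timeline plays at a rate of 1/Duration from CartStartOffset, mapping its Alpha to distance along the spline.
; Each update sets the actor's location from the spline in world space and its rotation in local space.
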(event `self.ReceiveBeginPlay`
  (if (`self.IsActive`)
    (`self.Move`)))

(event `Move`
  (bind _returnvalue (`KismetMathLibrary.Lerp` 0.0 (`SplineComponent.GetSplineLength` (`/Game/Blueprints/Vehicle/Track.Spline` (`self.Track`))) (`self.Alpha`)))
  (`TimelineComponent.SetPlayRate` (`self.Mover`) (/ 1.0 (`self.Duration`)))
  (`TimelineComponent.SetNewTime` (`self.Mover`) (`self.CartStartOffset`))
  (bind (_direction _alpha) (`Timeline|Mover`)
    (:`Update`
      (set `self.Alpha` _alpha)
      (`self.K2_SetActorLocationAndRotation` (`SplineComponent.GetLocationAtDistanceAlongSpline` (`/Game/Blueprints/Vehicle/Track.Spline` (`self.Track`)) _returnvalue "World") (`SplineComponent.GetRotationAtDistanceAlongSpline` (`/Game/Blueprints/Vehicle/Track.Spline` (`self.Track`)) _returnvalue "Local")))))

(fn `UserConstructionScript`)